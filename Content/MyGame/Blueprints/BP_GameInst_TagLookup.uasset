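; Game instance that serves weapon lookup data by gameplay tag and keeps a weapon inventory count.
; On Init it reads every WeaponDataTable row into two maps keyed by row name, one for animation index and one for joint target location.
; Getter functions convert a tag to its name to query those maps, printing an error on a miss.
; AddWeaponToInventory increments a per-tag quantity in InventoryMap.
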(event `self.ReceiveInit`
  ; DataTable을 통해 Weapon Tag와 int, 조인트 타겟을 매핑
  (bind _outrownames (`DataTableFunctionLibrary.GetDataTableRowNames` (`self.WeaponDataTable`)))
  (for _array_element _outrownames
    (bind _returnvalue (`|GetDataTableRow` (`self.WeaponDataTable`) _array_element)
      (:`then`
        (bind (_weaponindex _weaponname _tagweapontype _jointtargetlocation) (break `/Game/MyGame/Weapons/S_WeaponData` _returnvalue))
        (`BlueprintMapLibrary.Map_Add` (`self.WeaponTagToIndexMap`) _array_element _weaponindex)
        (`BlueprintMapLibrary.Map_Add` (`self.WeaponTagToJointMap`) _array_element _jointtargetlocation)))))

(fn `AddWeaponToInventory`
  (params (WeaponTag :type "GameplayTag Structure"))
  (locals (AddWeaponTag :type "GameplayTag Structure"))
  (bind (_value _returnvalue) (`BlueprintMapLibrary.Map_Find` (`self.InventoryMap`) (`local.AddWeaponTag`)))
  (set `local.AddWeaponTag` WeaponTag)
  (if _returnvalue
    ; 이미 아이템이 있으면 수량 +1
    (`BlueprintMapLibrary.Map_Add` (`self.InventoryMap`) (`local.AddWeaponTag`) (+ _value 1))
    (else
      ; 없으면 1로 추가
      (`BlueprintMapLibrary.Map_Add` (`self.InventoryMap`) (`local.AddWeaponTag`) 1))))

(fn `GetAnimIndexForTag`
  (params (InGamePlayTag :type "GameplayTag Structure"))
  (returns (OutIndex :type Integer))
  (bind (_value _returnvalue) (`BlueprintMapLibrary.Map_Find` (`self.WeaponTagToIndexMap`) (`BlueprintGameplayTagLibrary.GetTagName` InGamePlayTag)))
  (if _returnvalue
    (return _value)
    (else
      (`KismetSystemLibrary.PrintString` "BP_GameInst_TagLookup Error_GetAnimIndexForTag Error!!!!"))))

(fn `GetJointTargetVectorForTag`
  (params (InGamePlayTag :type "GameplayTag Structure"))
  (returns (JointTarget :type "Vector Structure"))
  (bind (_value _returnvalue) (`BlueprintMapLibrary.Map_Find` (`self.WeaponTagToJointMap`) (`BlueprintGameplayTagLibrary.GetTagName` InGamePlayTag)))
  (if _returnvalue
    (return _value)
    (else
      (`KismetSystemLibrary.PrintString` "BP_GameInst_TagLookup Error_GetJointTargetVectorForTag Error!!!!"))))