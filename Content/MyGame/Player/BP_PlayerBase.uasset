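; Base player character for a shooter, handling movement, stamina-limited sprint, crouch, jump, aiming, weapons, damage and HUD updates.
; Stats come from a tag-keyed data table, and a camera handler component blends aim-down-sights through a timeline.
; The inventory component handles pickup and switching, with weapon tags mapped through the GameInstance to animation indices for the AnimBP.
; Firing plays montages and passes camera-viewpoint trace hits to the weapon, while self-repeating delayed events drain and recover stamina.
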(event `self.ReceiveTick`
  (params (DeltaSeconds :type "Float (single-precision)")))

(event `self.ReceiveBeginPlay`
  ; 초기화
  (`|ExecutionSequence`
    (:`then_0`
      (set `self.PlayerController` (`GameplayStatics.GetPlayerController` 0))
      (bind _asbp_game_inst_tag_lookup (cast `/Game/MyGame/Blueprints/BP_GameInst_TagLookup` (`GameplayStatics.GetGameInstance`)))
      (set `self.Player BP Game Inst Tag Lookup Ref` _asbp_game_inst_tag_lookup)
      (bind _returnvalue (`|CreateWidget` "/Game/MyGame/UI/Player/WBP_PlayerFullHUD.WBP_PlayerFullHUD_C"))
      (bind _output_get (set `self.PlayerWidgetRef` _returnvalue))
      (`UserWidget.AddToViewport` _output_get 0)
      (`/Game/MyGame/UCameraHandlerComponent.InitializeCamera` (`self.UCameraHandlerComponent`) (`self.CommonSpringArm`) (`self.Camera`))
      (bind _returnvalue_2 (`|GetDataTableRow` (`self.PlayerDataTableInCharacter`) (`BlueprintGameplayTagLibrary.GetTagName` (`self.CurrentPlayerTag`)))
        (:`then`
          (bind _output_get_2 (set `self.PlayerStatsStruct` _returnvalue_2))
          (bind (_playerclass _playerwalkspeed _playerrunspeed _health _stamina) (break `/Game/MyGame/Player/S_PlayerCharacterStats` _output_get_2))
          (set `CharacterMovementComponent.MaxWalkSpeed` _playerwalkspeed (`self.CharacterMovement`))
          (set `self.PlayerMaxRunSpeed` _playerrunspeed)
          (set `self.PlayerCurrentHealth` _health)
          (set `self.PlayerCurrentStamina` _stamina)
          (`self.SetAnimationBluePrintObject`))))))

(event `Key|I`
  (params (Key :type "Key Structure")))

(event `EnhancedInput|/Game/MyGame/Player/Input/IA_Aim`
  (params (ActionValue :type Boolean) (ElapsedSeconds :type "Float (double-precision)") (TriggeredSeconds :type "Float (double-precision)") (InputAction :type "InputAction Object Reference" :default "/Game/MyGame/Player/Input/IA_Aim.IA_Aim"))
  ; 견착 모드
  (:`Started`
    (`/Engine/EditorBlueprintResources/StandardMacros.FlipFlop` :!label _label
      (:`A`
        (bind (_direction _blendalpha01) (`Timeline|TL_CameraBlendAlpha01` :!via `PlayFromStart` :!label _label_2)
          (:`Update`
            (switch `ETimelineDirection` _direction
              (:`Forward`
                ;; 정방향 = 1에 가까워 질 수록 ads(aimed)상태
                (`/Game/MyGame/UCameraHandlerComponent.SetADSCamera` (`self.UCameraHandlerComponent`) _blendalpha01)
                (set `self.bIsAimed` true))
              (:`Backward`
                (`/Game/MyGame/UCameraHandlerComponent.SetADSCamera` (`self.UCameraHandlerComponent`) _blendalpha01)
                (set `self.bIsAimed` false))))))
      (:`B`
        (goto _label_2 :!via `Reverse`))))
  (:`Canceled`
    (goto _label))
  (:`Completed`
    (goto _label)))

(event `EnhancedInput|/Game/MyGame/Player/Input/IA_Move`
  (params (ActionValue :type "Vector2D Structure") (ElapsedSeconds :type "Float (double-precision)") (TriggeredSeconds :type "Float (double-precision)") (InputAction :type "InputAction Object Reference" :default "/Game/MyGame/Player/Input/IA_Move.IA_Move"))
  (bind (_direction_x _direction_y) (`KismetMathLibrary.BreakVector2D` (`self.Direction`)))
  (bind (_returnvalue_roll _returnvalue_pitch _returnvalue_yaw) (`KismetMathLibrary.BreakRotator` (`Controller.GetControlRotation` (`GameplayStatics.GetPlayerController` 0))))
  ; 기본 이동
  ;; 걷기
  (:`Triggered`
    (set `self.Direction` (`KismetMathLibrary.MakeVector2D` ActionValue_Y ActionValue_X))
    (`self.AddMovementInput` (`KismetMathLibrary.GetForwardVector` (`KismetMathLibrary.MakeRotator` 0.0 0.0 _returnvalue_yaw)) _direction_x)
    (`self.AddMovementInput` (`KismetMathLibrary.GetRightVector` (`KismetMathLibrary.MakeRotator` _returnvalue_roll 0.0 _returnvalue_yaw)) _direction_y)))

(event `Key|NumPadZero`
  (params (Key :type "Key Structure")))

(event `EnhancedInput|/Game/MyGame/Player/Input/IA_Look`
  (params (ActionValue :type "Vector2D Structure") (ElapsedSeconds :type "Float (double-precision)") (TriggeredSeconds :type "Float (double-precision)") (InputAction :type "InputAction Object Reference" :default "/Game/MyGame/Player/Input/IA_Look.IA_Look"))
  ; 기본 이동
  ;; 회전
  (:`Triggered`
    (`self.AddControllerYawInput` ActionValue_X)
    (`self.AddControllerPitchInput` ActionValue_Y)))

(event `EnhancedInput|/Game/MyGame/Player/Input/IA_Interact`
  (params (ActionValue :type Boolean) (ElapsedSeconds :type "Float (double-precision)") (TriggeredSeconds :type "Float (double-precision)") (InputAction :type "InputAction Object Reference" :default "/Game/MyGame/Player/Input/IA_Interact.IA_Interact"))
  (bind _inventorymanagecomponent (`self.InventoryManageComponent`))
  (bind _weapon_magazine_size (`/Game/MyGame/Weapons/BluePrints/Equiped/BP_WeaponBase.Weapon Magazine Size` (`self.CurrentWeaponRef`)))
  ; 무기 시스템
  ;; 무기 해제/장착
  (:`Triggered`
    (if (== (`self.CurrentWeaponTag`) (struct :`TagName` "Weapon.Type.None"))
      ;;; 무기 미장착 상태면 마지막으로 꺼냈던 무기 장착
      (bind (_outcurrentweapon _ischange) (`/Game/MyGame/InventoryManageComponent.SwitchWeapon` _inventorymanagecomponent (`/Game/MyGame/InventoryManageComponent.CurrentSlotIndex` _inventorymanagecomponent) "Gun"))
      (if _ischange
        (`self.ChangeCurrentWeaponTag` _outcurrentweapon)
        ; ABP에 모션이 바뀜을 알림
        (`self.SendTagIndexToABP` :!label _label_3)
        (bind _outweapon (`/Game/MyGame/InventoryManageComponent.GetCurrentWeapon` (`self.InventoryManageComponent`)))
        (bind _asbp_weapon_base (cast `/Game/MyGame/Weapons/BluePrints/Equiped/BP_WeaponBase` _outweapon))
        (set `self.CurrentWeaponRef` _asbp_weapon_base)
        (message `/Game/MyGame/UI/Interfaces/BPI_HUDPlayerStatInterface.UpdateWeaponImage` (`self.PlayerWidgetRef`))
        (set `self.CurrentMagazine` _weapon_magazine_size)
        (`/Game/MyGame/UI/Interfaces/BPI_HUDPlayerStatInterface.UpdateWeaponMaxMagazine` (`self.PlayerWidgetRef`) _weapon_magazine_size)
        (`/Game/MyGame/UI/Interfaces/BPI_HUDPlayerStatInterface.UpdateWeaponCurrentMagazine` (`self.PlayerWidgetRef`) (`self.CurrentMagazine`)))
      (else
        ;;; 무기 해제
        (`/Game/MyGame/InventoryManageComponent.DestroyCurrentWeapon` (`self.InventoryManageComponent`))
        (set `self.CurrentWeaponTag` (struct :`TagName` "Weapon.Type.None"))
        (goto _label_3)))))

(event `EnhancedInput|/Game/MyGame/Player/Input/IA_Sprint`
  (params (ActionValue :type Boolean) (ElapsedSeconds :type "Float (double-precision)") (TriggeredSeconds :type "Float (double-precision)") (InputAction :type "InputAction Object Reference" :default "/Game/MyGame/Player/Input/IA_Sprint.IA_Sprint"))
  ; 기본 이동
  ;; 달리기
  (:`Started`
    (`/Engine/EditorBlueprintResources/StandardMacros.FlipFlop` :!label _label_4
      (:`A`
        (`self.OnSprint`)
        (`self.Consume Stamina`))
      (:`B`
        (`self.OffSprint`)
        (`self.Recovery Stamina`))))
  (:`Completed`
    (goto _label_4)))

(event `Consume Stamina`
  (bind (_playerstatsstruct_playerclass _playerstatsstruct_playerwalkspeed _playerstatsstruct_playerrunspeed _playerstatsstruct_health _playerstatsstruct_stamina) (break `/Game/MyGame/Player/S_PlayerCharacterStats` (`self.PlayerStatsStruct`)))
  ; 기본 이동
  ;; 달리기
  (bind _output_get (set `self.PlayerCurrentStamina` (`KismetMathLibrary.FClamp` (- (`self.PlayerCurrentStamina`) 1.0) 0.0 _playerstatsstruct_stamina)))
  (message `/Game/MyGame/UI/Interfaces/BPI_HUDPlayerStatInterface.UpdatePlayerStamina` (`self.PlayerWidgetRef`) _output_get _playerstatsstruct_stamina)
  (if (== _output_get 0.0)
    (`self.OffSprint`)
    (elif (`self.bIsSprint`)
      (`KismetSystemLibrary.Delay` 0.1)
      (`self.Consume Stamina`))))

(event `Recovery Stamina`
  (bind (_playerstatsstruct_playerclass _playerstatsstruct_playerwalkspeed _playerstatsstruct_playerrunspeed _playerstatsstruct_health _playerstatsstruct_stamina) (break `/Game/MyGame/Player/S_PlayerCharacterStats` (`self.PlayerStatsStruct`)))
  ; 기본 이동
  ;; 달리기
  (bind _output_get (set `self.PlayerCurrentStamina` (`KismetMathLibrary.FClamp` (+ (`self.PlayerCurrentStamina`) 1.0) 0.0 _playerstatsstruct_stamina)))
  (message `/Game/MyGame/UI/Interfaces/BPI_HUDPlayerStatInterface.UpdatePlayerStamina` (`self.PlayerWidgetRef`) _output_get _playerstatsstruct_stamina)
  (if (== _output_get _playerstatsstruct_stamina)
    _
    (elif (not (`self.bIsSprint`))
      (`KismetSystemLibrary.Delay` 0.2)
      (`self.Recovery Stamina`))))

(event `EnhancedInput|/Game/MyGame/Player/Input/IA_Crouch`
  (params (ActionValue :type Boolean) (ElapsedSeconds :type "Float (double-precision)") (TriggeredSeconds :type "Float (double-precision)") (InputAction :type "InputAction Object Reference" :default "/Game/MyGame/Player/Input/IA_Crouch.IA_Crouch"))
  (bind _charactermovement (`self.CharacterMovement`))
  ; 기본 이동
  ;; 앉기
  (:`Triggered`
    (if (not (`NavMovementInterface.IsFalling` _charactermovement))
      (if (`NavMovementInterface.IsCrouching` _charactermovement)
        (`self.UnCrouch`)
        (else
          (`self.Crouch`))))))

(event `EnhancedInput|/Game/MyGame/Player/Input/IA_Jump`
  (params (ActionValue :type Boolean) (ElapsedSeconds :type "Float (double-precision)") (TriggeredSeconds :type "Float (double-precision)") (InputAction :type "InputAction Object Reference" :default "/Game/MyGame/Player/Input/IA_Jump.IA_Jump"))
  ; 기본 이동
  ;; 점프
  (:`Started`
    (if (not (`NavMovementInterface.IsFalling` (`self.CharacterMovement`)))
      (set `self.bIsAimed` false)
      (`/Game/MyGame/UCameraHandlerComponent.SetADSCamera` (`self.UCameraHandlerComponent`) 0.0)
      (`self.Jump`))))

(event `EnhancedInput|/Game/MyGame/Player/Input/IA_WeaponSlot1`
  (params (ActionValue :type Boolean) (ElapsedSeconds :type "Float (double-precision)") (TriggeredSeconds :type "Float (double-precision)") (InputAction :type "InputAction Object Reference" :default "/Game/MyGame/Player/Input/IA_WeaponSlot1.IA_WeaponSlot1"))
  ; 무기 시스템
  ;; 무기 스위치
  (:`Triggered`
    (bind (_outcurrentweapon _ischange) (`/Game/MyGame/InventoryManageComponent.SwitchWeapon` (`self.InventoryManageComponent`) 0 "Gun"))
    (if _ischange
      (`self.ChangeCurrentWeaponTag` _outcurrentweapon)
      (goto _label_3))))

(event `EnhancedInput|/Game/MyGame/Player/Input/IA_WeaponSlot2`
  (params (ActionValue :type Boolean) (ElapsedSeconds :type "Float (double-precision)") (TriggeredSeconds :type "Float (double-precision)") (InputAction :type "InputAction Object Reference" :default "/Game/MyGame/Player/Input/IA_WeaponSlot2.IA_WeaponSlot2"))
  ; 무기 시스템
  ;; 무기 스위치
  (:`Triggered`
    (bind (_outcurrentweapon _ischange) (`/Game/MyGame/InventoryManageComponent.SwitchWeapon` (`self.InventoryManageComponent`) 1 "Gun"))
    (if _ischange
      (`self.ChangeCurrentWeaponTag` _outcurrentweapon)
      (goto _label_3))))

(event `self.ReceiveActorBeginOverlap`
  (params (OtherActor :type "Actor Object Reference"))
  (bind _output (`|GetArrayItem` (`self.GetOverlappingActors` "/Game/MyGame/Weapons/BluePrints/PickUp/BP_WeaponItemPickup.BP_WeaponItemPickup_C")))
  ; 아이템에 다가갈 시에 먹을 수 있으면 인벤토리에 추가
  (`/Engine/EditorBlueprintResources/StandardMacros.IsValid` _output
    (:`Is Valid`
      (`/Game/MyGame/InventoryManageComponent.PickUpWeapon` (`self.InventoryManageComponent`) _output)
      (message `/Game/MyGame/Interfaces/BPI_WeaponSystem.OnPickUp` _output))))

(event `EnhancedInput|/Game/MyGame/Player/Input/IA_WeaponNext`
  (params (ActionValue :type Boolean) (ElapsedSeconds :type "Float (double-precision)") (TriggeredSeconds :type "Float (double-precision)") (InputAction :type "InputAction Object Reference" :default "/Game/MyGame/Player/Input/IA_WeaponNext.IA_WeaponNext"))
  ; 무기 시스템
  ;; 무기 스위치
  (:`Started`
    (bind _returnvalue (`self.SetWeaponSlotIndex` 1))
    (bind (_outcurrentweapon _ischange) (`/Game/MyGame/InventoryManageComponent.SwitchWeapon` (`self.InventoryManageComponent`) _returnvalue "Gun"))
    (if _ischange
      (`self.ChangeCurrentWeaponTag` _outcurrentweapon)
      (goto _label_3))))

(event `EnhancedInput|/Game/MyGame/Player/Input/IA_WeaponPrevious`
  (params (ActionValue :type Boolean) (ElapsedSeconds :type "Float (double-precision)") (TriggeredSeconds :type "Float (double-precision)") (InputAction :type "InputAction Object Reference" :default "/Game/MyGame/Player/Input/IA_WeaponPrevious.IA_WeaponPrevious"))
  ; 무기 시스템
  ;; 무기 스위치
  (:`Started`
    (bind _returnvalue (`self.SetWeaponSlotIndex` -1))
    (bind (_outcurrentweapon _ischange) (`/Game/MyGame/InventoryManageComponent.SwitchWeapon` (`self.InventoryManageComponent`) _returnvalue "Gun"))
    (if _ischange
      (`self.ChangeCurrentWeaponTag` _outcurrentweapon)
      (goto _label_3))))

(event `EnhancedInput|/Game/MyGame/Player/Input/IA_MouseLeftAttack`
  (params (ActionValue :type Boolean) (ElapsedSeconds :type "Float (double-precision)") (TriggeredSeconds :type "Float (double-precision)") (InputAction :type "InputAction Object Reference" :default "/Game/MyGame/Player/Input/IA_MouseLeftAttack.IA_MouseLeftAttack"))
  (bind _currentweaponref (`self.CurrentWeaponRef`))
  ; 공격
  (:`Ongoing`
    (`/Engine/EditorBlueprintResources/StandardMacros.IsValid` (`/Game/MyGame/InventoryManageComponent.CurrentWeapon` (`self.InventoryManageComponent`))
      (:`Is Valid`
        (if (!= (`self.CurrentMagazine`) 0)
          (set `self.bIsFiring` true)
          (`|ExecutionSequence`
            (:`then_0`
              (`KismetSystemLibrary.Delay` (/ 1.0 (`/Game/MyGame/Weapons/BluePrints/Equiped/BP_WeaponBase.Weapon Attack Count Per Second` _currentweaponref)))
              (if (`self.bIsAimed`)
                (`|PlayMontage` (`self.Mesh`) "/Game/Animations/MyAni/RifleAnims/RealAnimations/Fire_Reload_Equip_Jump/AM_Rifle_Fire_Aim.AM_Rifle_Fire_Aim" (`/Game/MyGame/Weapons/BluePrints/Equiped/BP_WeaponBase.Weapon Attack Count Per Second` (`self.CurrentWeaponRef`))
                  (:`then`
                    _))
                (else
                  (`|PlayMontage` (`self.Mesh`) "/Game/Animations/MyAni/RifleAnims/RealAnimations/Fire_Reload_Equip_Jump/AM_Rifle_Fire.AM_Rifle_Fire" (`/Game/MyGame/Weapons/BluePrints/Equiped/BP_WeaponBase.Weapon Attack Count Per Second` (`self.CurrentWeaponRef`))
                    (:`then`
                      _))))
              (bind (_ishit _outhit) (`self.OnTraceHitLocation`))
              (`/Game/MyGame/Weapons/BluePrints/Equiped/BP_WeaponBase.Fire` _currentweaponref _ishit _outhit)
              (`self.UpdateMagazineUI`)))))))
  (:`Canceled`
    (set `self.bIsFiring` false :!label _label_5))
  (:`Completed`
    (goto _label_5)))

(event `self.ReceiveAnyDamage`
  (params (Damage :type "Float (single-precision)") (DamageType :type "DamageType Object Reference") (InstigatedBy :type "Controller Object Reference") (DamageCauser :type "Actor Object Reference"))
  (bind (_playerstatsstruct_playerclass _playerstatsstruct_playerwalkspeed _playerstatsstruct_playerrunspeed _playerstatsstruct_health) (break `/Game/MyGame/Player/S_PlayerCharacterStats` (`self.PlayerStatsStruct`)))
  (bind _returnvalue (- (`self.PlayerCurrentHealth`) Damage))
  ; 데미지 처리
  (bind _output_get (set `self.bIsDead` (<= _returnvalue 0.0)))
  (if (not _output_get)
    (bind _output_get_2 (set `self.PlayerCurrentHealth` _returnvalue))
    (message `/Game/MyGame/UI/Interfaces/BPI_HUDPlayerStatInterface.UpdatePlayerHealth` (`self.PlayerWidgetRef`) _output_get_2 _playerstatsstruct_health)))

(event `UpdateMagazineUI`
  (bind _output_get (set `self.CurrentMagazine` (`KismetMathLibrary.Clamp` (- (`self.CurrentMagazine`) 1) 0 (`/Game/MyGame/Weapons/BluePrints/Equiped/BP_WeaponBase.Weapon Magazine Size` (`self.CurrentWeaponRef`)))))
  (`/Game/MyGame/UI/Interfaces/BPI_HUDPlayerStatInterface.UpdateWeaponCurrentMagazine` (`self.PlayerWidgetRef`) _output_get))

(fn `GetLeftHandSocketTransform`
  (returns (LeftHandWeaponSocketTransform :type "Transform Structure"))
  (`/Engine/EditorBlueprintResources/StandardMacros.IsValid` (`self.CurrentWeaponRef`)
    (:`Is Valid`
      (bind _sockettransform (message `/Game/MyGame/Interfaces/BPI_GetWeaponInform.GetWeaponSkeletonSocket` (`self.CurrentWeaponRef`)))
      (bind (_outposition _outrotation) (`SkinnedMeshComponent.TransformToBoneSpace` (`self.Mesh`) "hand_r" (.location _sockettransform) (.rotation _sockettransform)))
      (return (`KismetMathLibrary.MakeTransform` _outposition _outrotation)))))

(fn `GetPlayerTag`
  (returns (OutTag :type "GameplayTag Structure"))
  (return (`self.CurrentPlayerTag`)))

(fn `OffSprint`
  (bind (_playerstatsstruct_playerclass _playerstatsstruct_playerwalkspeed) (break `/Game/MyGame/Player/S_PlayerCharacterStats` (`self.PlayerStatsStruct`)))
  (set `CharacterMovementComponent.MaxWalkSpeed` _playerstatsstruct_playerwalkspeed (`self.CharacterMovement`))
  (set `self.bIsSprint` false))

(fn `OnSprint`
  (bind (_playerstatsstruct_playerclass _playerstatsstruct_playerwalkspeed _playerstatsstruct_playerrunspeed) (break `/Game/MyGame/Player/S_PlayerCharacterStats` (`self.PlayerStatsStruct`)))
  (set `CharacterMovementComponent.MaxWalkSpeed` _playerstatsstruct_playerrunspeed (`self.CharacterMovement`))
  (set `self.bIsSprint` true))

(fn `OnTraceHitLocation`
  (returns (IsHit :type Boolean) (OutHit :type "HitResult Structure"))
  (locals (HitLocation :type "Vector Structure" :default (0.0 0.0 0.0)))
  (bind (_location _rotation) (`Controller.GetPlayerViewPoint` (`GameplayStatics.GetPlayerController` 0)))
  (bind (_outhit _returnvalue) (`KismetSystemLibrary.LineTraceSingle` _location (+ _location (* (`KismetMathLibrary.GetForwardVector` _rotation) (`/Game/MyGame/Weapons/BluePrints/Equiped/BP_WeaponBase.Weapon Range` (`self.CurrentWeaponRef`)))) "TraceTypeQuery3"))
  (return _returnvalue _outhit))

(fn `SendTagIndexToABP`
  (bind _outindex (`/Game/MyGame/Blueprints/BP_GameInst_TagLookup.GetAnimIndexForTag` (`self.Player BP Game Inst Tag Lookup Ref`) (`self.CurrentWeaponTag`)))
  (bind _output_get (set `self.TagAnimIndex` _outindex))
  (message `/Game/MyGame/Interfaces/BPI_WeaponSystem.OnChangeWeapon` (`self.As ABP Player Character`) _output_get (`self.CurrentWeaponTag`)))

(fn `SetWalkSpeed`
  (params (InSpeed :type "Float (double-precision)")))

(fn `SetWeaponSlotIndex`
  (params (InAddIndex :type Integer))
  (returns (ReturnValue :type Integer))
  (bind _returnvalue (`KismetArrayLibrary.Array_Length` (`/Game/MyGame/InventoryManageComponent.WeaponsInSlot` (`self.InventoryManageComponent`))))
  (bind _output_get (set `/Game/MyGame/InventoryManageComponent.CurrentSlotIndex` (mod (+ (+ (`/Game/MyGame/InventoryManageComponent.CurrentSlotIndex` (`self.InventoryManageComponent`)) InAddIndex) _returnvalue) _returnvalue) (`self.InventoryManageComponent`)))
  (return _output_get))

(fn `UserConstructionScript`)