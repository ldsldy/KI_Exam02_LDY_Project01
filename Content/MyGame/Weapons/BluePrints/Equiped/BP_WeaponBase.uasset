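; Base Blueprint for equipped weapons, handling stats, firing, damage and effects.
; BeginPlay loads stats from a DataTable row named by the weapon's gameplay tag.
; Fire takes the caller's hit, re-traces from the muzzle toward it (or the stored location), and on a hit applies point damage and spawns a rifle projectile.
; Fire also plays a rate-scaled rifle montage and muzzle-flash Niagara; getters expose tag and left-hand socket, while GetWeaponStats returns zeros.
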(event `self.ReceiveBeginPlay`
  (bind _returnvalue (`|GetDataTableRow` (`.DataTable` (break `DataTableRowHandle` (`self.WeaponDataTable`))) (`BlueprintGameplayTagLibrary.GetTagName` (`self.WeaponTag`)))
    (:`then`
      (bind (_weaponindex _weaponname _tagweapontype _jointtargetlocation _damage _magazinesize _pickupweaponclass _equipweaponclass _attackcountpersecond _range) (break `/Game/MyGame/Weapons/S_WeaponData` _returnvalue))
      (set `self.WeaponDamage` _damage)
      (set `self.Weapon Magazine Size` _magazinesize)
      (set `self.Weapon Attack Count Per Second` _attackcountpersecond)
      (set `self.Weapon Range` _range)
      (set `self.Current Magzine` (`self.Weapon Magazine Size`)))))

(event `Fire`
  (params (IsHit :type Boolean) (HitInfo :type "HitResult Structure"))
  (bind (_returnvalue_location _returnvalue_rotation) (`KismetMathLibrary.BreakTransform` (`SceneComponent.GetSocketTransform` (`self.Weapon`) "Muzzle" "RTS_World")))
  (`self.OnTraceAndHit` HitInfo IsHit)
  (`|PlayMontage` (`self.Weapon`) "/Game/Weapons/Rifle/Animations/AM_Weap_Rifle_Fire.AM_Weap_Rifle_Fire" (`self.Weapon Attack Count Per Second`)
    (:`then`
      (`NiagaraFunctionLibrary.SpawnSystemAttached` "/Game/100_MuzzleFlashes/Muzzle_Flash/MuzzleFlash_Niagara/P_MuzzleFlash3.P_MuzzleFlash3" (`self.Weapon`) "Muzzle" (+ _returnvalue_location (* (`KismetMathLibrary.GetForwardVector` _returnvalue_rotation) 5.0)) (`KismetMathLibrary.MakeRotator` (.roll _returnvalue_rotation) (.pitch _returnvalue_rotation) (+ (.yaw _returnvalue_rotation) -90.0)) "KeepWorldPosition" true))))

(fn `GetWeaponSkeletonSocket`
  (returns (SocketTransform :type "Transform Structure"))
  (return (`SceneComponent.GetSocketTransform` (`self.Weapon`) "LeftHand_Weapon_Socket" "RTS_World")))

(fn `GetWeaponStats`
  (returns (FireRate :type "Float (double-precision)") (Damage :type "Float (double-precision)"))
  (return 0.0 0.0))

(fn `GetWeaponTag`
  (returns (WeaponTag :type "GameplayTag Structure"))
  (return (`self.WeaponTag`)))

(fn `GetWeaponTagName`
  (returns (TagName :type Name))
  (return (`BlueprintGameplayTagLibrary.GetTagName` (`self.WeaponTag`))))

(fn `OnTraceAndHit`
  (params (InHit :type "HitResult Structure") (IsHit :type Boolean))
  (locals (HitLocation :type "Vector Structure" :default (0.0 0.0 0.0)))
  (bind _returnvalue (`SceneComponent.GetSocketLocation` (`self.Weapon`) "Muzzle"))
  (if IsHit
    (set `local.HitLocation` (`.Location` (`GameplayStatics.BreakHitResult` InHit)))
    (else
      (set `local.HitLocation` (`local.HitLocation`))))
  ; 맞았으면 그 지점으로 트레이스를 맞은 오브젝트가 없으면 트레이스 끝 점으로 트레이스
  (bind (_outhit _returnvalue_2) (`KismetSystemLibrary.LineTraceSingle` :`Start` (`SceneComponent.GetSocketLocation` (`self.Weapon`) "Muzzle") :`End` (`local.HitLocation`) :`TraceChannel` "TraceTypeQuery3" :`TraceColor` (struct :`G` 0.117609 :`B` 1.0 :`A` 1.0) :`DrawTime` 3.0))
  (if _returnvalue_2
    (bind (_bblockinghit _binitialoverlap _time _distance _location _impactpoint _normal _impactnormal _physmat _hitactor _hitcomponent _hitbonename _bonename _hititem _elementindex _faceindex _tracestart) (`GameplayStatics.BreakHitResult` _outhit))
    (`GameplayStatics.ApplyPointDamage` _hitactor (`self.WeaponDamage`) _tracestart _outhit (`GameplayStatics.GetPlayerController` 0))
    ; !!!총알 종류 테이블에 추가하기
    (`|SpawnActorFromClass` "/Game/MyGame/Projectilees/PlayerProjectile/BP_RifleProjectile.BP_RifleProjectile_C" (`KismetMathLibrary.MakeTransform` (+ (* (`self.GetActorForwardVector` (`GameplayStatics.GetPlayerController` 0)) 15.0) _returnvalue) (`KismetMathLibrary.FindLookAtRotation` _returnvalue (`local.HitLocation`))) "Undefined" "MultiplyWithRoot" null null)
    (return)))

(fn `UserConstructionScript`)