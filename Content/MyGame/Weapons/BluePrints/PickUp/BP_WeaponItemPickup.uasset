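; BP_WeaponItemPickup is a weapon pickup actor that is identified by a gameplay tag and destroys itself on OnPickUp.
; Its construction script traces downward on Visibility and, on a hit, snaps the actor slightly above the ground.
; It then looks up the tag's name as a WeaponData table row, but leaves the result unused.
; Getters expose the tag and its name, while GetWeaponStats returns only zeros.
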(event `/Game/MyGame/Interfaces/BPI_WeaponSystem.OnPickUp`
  (`self.K2_DestroyActor`))

(fn `GetWeaponStats`
  (returns (FireRate :type "Float (double-precision)") (Damage :type "Float (double-precision)"))
  (return 0.0 0.0))

(fn `GetWeaponTag`
  (returns (WeaponTag :type "GameplayTag Structure"))
  (return (`self.WeaponTag`)))

(fn `GetWeaponTagName`
  (returns (TagName :type Name))
  (return (`BlueprintGameplayTagLibrary.GetTagName` (`self.WeaponTag`))))

(fn `UserConstructionScript`
  (bind _returnvalue (`self.K2_GetActorLocation`))
  ; 생성될 떄 땅 바닥에 생성
  (bind _outhit (`KismetSystemLibrary.LineTraceSingle` _returnvalue (- _returnvalue (0.0 0.0 500.0)) "TraceTypeQuery1" true))
  (bind (_bblockinghit _binitialoverlap _time _distance _location) (`GameplayStatics.BreakHitResult` _outhit))
  (if _bblockinghit
    (`self.K2_SetActorLocation` (+ _location (0.0 0.0 20.0)))
    (bind _returnvalue_2 (`|GetDataTableRow` (`.DataTable` (break `DataTableRowHandle` (`self.WeaponData`))) (`BlueprintGameplayTagLibrary.GetTagName` (`self.WeaponTag`))))))