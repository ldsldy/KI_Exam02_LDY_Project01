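; AI controller for the flying ranged enemy that runs its behavior tree and reacts to perceiving the player.
; On spawn it caches the controlled pawn and its tag container.
; Perception updates filter actors by player tag, passing stimuli from the first updated actor to sight handling.
; A successful sense stores locations and switches Patrol or Investigate to Chase at chase fly speed; a data-table sight-range lookup is unconnected.
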(event `self.ReceiveBeginPlay`
  (`self.RunBehaviorTree` "/Game/MyGame/Enemies/Ranged_Air_Enemy/BT_Fly_Range_Enemy.BT_Fly_Range_Enemy"))

(event `/Game/Interfaces/BPI_SpawnableEnemy.OnSpawn`
  (bind _asbp_fly_range_enemy (cast `/Game/MyGame/Enemies/Ranged_Air_Enemy/BP_Fly_Range_Enemy` (`self.K2_GetPawn`)))
  (set `self.AC_BP Fly Range Enemy` _asbp_fly_range_enemy)
  (bind _inenemytag (message `/Game/Interfaces/BPI_ProviderEnemyInfo.GetEnemyTagContainer` (`self.K2_GetPawn`)))
  (set `self.AC_EnemyTagContainer` _inenemytag))

(event `self.AIPerception.OnPerceptionUpdated`
  (params (UpdatedActors :type "Array of Actor Object Reference (by ref)"))
  (for (_array_element _array_index) UpdatedActors
    (bind _outtag (message `/Game/Interfaces/BPI_ProviderCharacterInfo.GetPlayerTag` _array_element))
    (if (`BlueprintGameplayTagLibrary.HasTag` _outtag (struct :`TagName` "PlayerCharacter.Name"))
      (bind _info (`AIPerceptionComponent.GetActorsPerception` (`self.AIPerception`) _array_element))
      (for _array_element_2 (`.LastSensedStimuli` (break `ActorPerceptionBlueprintInfo` _info))
        (set `self.ActiveSense` _array_element_2)
        (switch `int` _array_index
          (:`0`
            (`self.SightSense`)))))))

(event `SightSense`
  (bind _ac_bp_fly_range_enemy (`self.AC_BP Fly Range Enemy`))
  (bind _ac_bp_fly_range_enemy_2 (`self.AC_BP Fly Range Enemy`))
  (bind (_age _expirationage _strength _stimuluslocation _receiverlocation _tag _bsuccessfullysensed) (break `AIStimulus` (`self.ActiveSense`)))
  (if _bsuccessfullysensed
    (set `self.Stimulus Location` _stimuluslocation)
    (set `self.Receiver Location` _receiverlocation)
    ; 나중에 게임 플레이 태그로 바꾸기
    (`KismetSystemLibrary.PrintString` "Chase")
    (switch `/Game/MyGame/Enemies/Ranged_Air_Enemy/E_StandStateEnemy` (`/Game/MyGame/Enemies/Ranged_Air_Enemy/BP_Fly_Range_Enemy.AIState` _ac_bp_fly_range_enemy)
      (:`NewEnumerator0`
        _)
      (:`NewEnumerator3`
        _))
    (set `/Game/MyGame/Enemies/Ranged_Air_Enemy/BP_Fly_Range_Enemy.AIState` "NewEnumerator1" _ac_bp_fly_range_enemy)
    (set `CharacterMovementComponent.MaxFlySpeed` (`/Game/MyGame/Enemies/BP_EnemyBase.Chase Speed` _ac_bp_fly_range_enemy_2) (`Character.CharacterMovement` _ac_bp_fly_range_enemy_2))))

(fn `UserConstructionScript`)