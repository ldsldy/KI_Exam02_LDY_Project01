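; BP_Enemy_Ranged_Air is the Blueprint for a ranged flying enemy, adding a random patrol destination picker to its parent class.
; GetRamdomLocation picks a random XY offset from the actor's current position at the same height, retrying up to ten times until it falls within PatrolRaius.
; The radius is measured from the current location rather than a fixed origin, and failure returns the current location.
; Its event graph and construction script only call the parent.
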(event `self.ReceiveBeginPlay`
  (`parent.ReceiveBeginPlay`))

(fn `GetRamdomLocation`
  (returns (OutLocation :type "Vector Structure"))
  (locals (TryIndex :type Integer))
  (bind (_currentlocation_x _currentlocation_y _currentlocation_z) (`KismetMathLibrary.BreakVector` (`self.CurrentLocation`)))
  (set `local.TryIndex` 0)
  (set `self.CurrentLocation` (`self.K2_GetActorLocation`))
  (set `self.TargetLocation` (`KismetMathLibrary.MakeVector` (+ (`KismetMathLibrary.RandomFloatInRange` -1000.0 1000.0) _currentlocation_x) (+ (`KismetMathLibrary.RandomFloatInRange` -1000.0 1000.0) _currentlocation_y) _currentlocation_z) :!label _label)
  (if (> (`KismetMathLibrary.Abs` (`KismetMathLibrary.VSize` (- (`self.CurrentLocation`) (`self.TargetLocation`)))) (`self.PatrolRaius`))
    ; 실패는 10번까지
    (bind _result (`/Engine/EditorBlueprintResources/StandardMacros.IncrementInt` (`local.TryIndex`))
      (:`  `
        (if (< _result 10)
          (goto _label)
          (else
            ; 최종 실패면 이동 X
            (return (`self.CurrentLocation`))))))
    (else
      ; 성공하면 그 위치로
      (return (`self.TargetLocation`)))))

(fn `UserConstructionScript`
  (`parent.UserConstructionScript`))