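; Boss AI controller that starts the boss behavior tree and blackboard on BeginPlay or OnSpawn.
; Perception updates are filtered to the player pawn, with stimulus array index selecting the sight or damage handler.
; Both handlers share one path: a successfully sensed stimulus changes the boss state and writes EnemyState and TargetActor to the blackboard.
; Failed or lost stimuli leave the state and target unchanged.
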(event `self.ReceiveBeginPlay`
  (`self.RunBehaviorTree` "/Game/MyGame/Enemies/Enemy/Boss/AI/BT_Boss.BT_Boss" :!label _label)
  (bind _blackboardcomponent (`self.UseBlackboard` "/Game/MyGame/Enemies/Enemy/Boss/AI/BB_Boss.BB_Boss"))
  (set `self.BossBlackboardComponent` _blackboardcomponent))

(event `/Game/MyGame/Interfaces/BPI_SpawnableEnemy.OnSpawn`
  (goto _label))

(event `self.AIPerception.OnPerceptionUpdated`
  (params (UpdatedActors :type "Array of Actor Object Reference (by ref)"))
  (for _array_element UpdatedActors
    (if (== _array_element (`GameplayStatics.GetPlayerPawn` 0))
      (bind _info (`AIPerceptionComponent.GetActorsPerception` (`self.AIPerception`) _array_element))
      (for (_array_element_2 _array_index) (`.LastSensedStimuli` (break `ActorPerceptionBlueprintInfo` _info))
        (set `self.ActiveSense` _array_element_2)
        (switch `int` _array_index
          (:`0`
            (`self.Boss Sight Sense`))
          (:`1`
            (`self.Damage Sense`)))))))

(event `Damage Sense`
  (if (`.bSuccessfullySensed` (break `AIStimulus` (`self.ActiveSense`))) :!label _label_2
    (bind _output_get (set `self.BossState` "NewEnumerator1"))
    (`BlackboardComponent.SetValueAsEnum` (`self.BossBlackboardComponent`) "EnemyState" _output_get)
    (`BlackboardComponent.SetValueAsObject` (`self.BossBlackboardComponent`) "TargetActor" (`GameplayStatics.GetPlayerPawn` 0))))

(event `Boss Sight Sense`
  (goto _label_2))

(fn `UserConstructionScript`)