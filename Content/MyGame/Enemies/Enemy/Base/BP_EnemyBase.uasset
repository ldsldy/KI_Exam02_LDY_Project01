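; Base enemy Blueprint that loads its stats from DT_EnemyDataTable by name tag and handles damage and death.
; BeginPlay applies walk speed, messages the AI controller for its tag container, caches the player and, under a flying ranged controller, registers itself in the blackboard as DroneActor.
; Point damage from Enemy-tagged causers is ignored; other hits spawn Niagara sparks and reduce health, with lethal hits playing a death montage before destroying the actor.
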(event `self.ReceiveBeginPlay`
  (`self.SetInitEnemyStats`)
  (set `CharacterMovementComponent.MaxWalkSpeed` (`self.Enemy Walk Speed`) (`self.CharacterMovement`))
  (message `/Game/MyGame/Interfaces/BPI_ProviderEnemyInfo.GetEnemyTagContainer` (`AIBlueprintHelperLibrary.GetAIController` self))
  (bind _asbp_player_base (cast `/Game/MyGame/Player/BP_PlayerBase` (`GameplayStatics.GetPlayerPawn` 0)))
  (set `self.PlayerRef` _asbp_player_base)
  (bind _asbp_ac_fly_range_enemy (cast `/Game/MyGame/Enemies/Enemy/Range/Ranged_Air_Enemy/Blueprints/BP_AC_Fly_Range_Enemy` (`self.GetController`)))
  (bind _output_get (set `self.AIController Ranged AIr Enemy` _asbp_ac_fly_range_enemy))
  (bind _blackboardcomponent (`AIController.UseBlackboard` _output_get "/Game/MyGame/Enemies/Enemy/Range/Ranged_Air_Enemy/BB_Fly_Range_Enemy.BB_Fly_Range_Enemy"))
  (bind _output_get_2 (set `self.Blackboard Component` _blackboardcomponent))
  (`BlackboardComponent.SetValueAsObject` _output_get_2 "DroneActor" self))

(event `self.ReceivePointDamage`
  (params (Damage :type "Float (single-precision)") (DamageType :type "DamageType Object Reference") (HitLocation :type "Vector Structure") (HitNormal :type "Vector Structure") (HitComponent :type "PrimitiveComponent Object Reference") (BoneName :type Name) (ShotFromDirection :type "Vector Structure") (InstigatedBy :type "Controller Object Reference") (DamageCauser :type "Actor Object Reference") (HitInfo :type "HitResult Structure (by ref)"))
  (bind _returnvalue (- (`self.Enemy Health`) Damage))
  ; 데미지 처리
  ;; 공격한 상대가 같은 Enemy태그를 가지고 있으면 데미지 무시
  (bind _returnvalue_2 (message `GameplayTagAssetInterface.HasMatchingGameplayTag` DamageCauser (struct :`TagName` "Enemy")))
  (if (not _returnvalue_2)
    (bind _returnvalue_3 (`NiagaraFunctionLibrary.SpawnSystemAtLocation` "/Game/RealisticSparkVersion2/Niagara/System/DirectionBurst/NS_DeathSplitSpark_Loop_RandDirection.NS_DeathSplitSpark_Loop_RandDirection" HitLocation (struct) (0.5 0.5 0.5) true true "AutoRelease"))
    ;; 상대의 공격이면 데미지 입음
    (`KismetSystemLibrary.PrintString` (`KismetStringLibrary.BuildString_Object` "Spawn" "" _returnvalue_3))
    (set `self.Enemy Health` _returnvalue)
    (bind _output_get (set `self.bIsDead` (<= _returnvalue 0.0)))
    ;;; 사망 모션
    (if _output_get
      (`|PlayMontage` (`self.Mesh`) (`self.EnemyDeathMontage`)
        (:`OnCompleted`
          (`self.K2_DestroyActor`))))))

(fn `UserConstructionScript`)