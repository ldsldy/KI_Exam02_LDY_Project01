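; Base Blueprint for a ranged enemy that strafes sideways while turning toward the player and firing bursts of projectiles.
; StartAttackRangeEnemy drives movement and alternates attacks with a delta-time reload cooldown.
; A timed loop macro aims the Muzzle at the player's spine socket and plays the attack montage once per round, paced by attack rate.
; A separate OnFireEffect event spawns the projectile at the Muzzle with the enemy as owner.
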(event `RangeEnemyOnFireEvent`
  ; 플레이어 방향으로 발사를 명령하는 이벤트
  (set `self.bIsAttacking` true)
  (`/Game/MyGame/Enemies/Macros/DelayMacros.EachLoopWithMacros` 1 (`self.Enemy Ammo Capaciy`) (/ 1.0 (`self.EnemyAttackCountPerSecond`))
    (:`LoopBody`
      (`self.FindLookAtPlayer`)
      (if (`self.bIsDead`)
        _
        (elif (not (`/Game/MyGame/Player/BP_PlayerBase.bIsDead` (`self.PlayerRef`)))
          (`|PlayMontage` (`self.Mesh`) (`self.RangeEnemyAttackMontage`) (`self.EnemyAttackCountPerSecond`)))))
    (:`Complete`
      (set `self.bIsReloading` true)
      (set `self.bIsAttacking` false))))

(event `OnFireEffect`
  (bind (_returnvalue_location _returnvalue_rotation) (`KismetMathLibrary.BreakTransform` (`SceneComponent.K2_GetComponentToWorld` (`self.Muzzle`))))
  ; 실제 발사체 발사, 소리, 효과 이벤트
  ;; 발사체에 자신의 정보를 담아서 스폰
  (bind _returnvalue (`|SpawnActorFromClass` (`self.EnemyProjectile`) (`KismetMathLibrary.MakeTransform` _returnvalue_location _returnvalue_rotation) "Undefined" "MultiplyWithRoot" null null))
  (`self.SetOwner` _returnvalue self))

(fn `FindLookAtPlayer`
  (`SceneComponent.K2_SetWorldRotation` (`self.Muzzle`) (`KismetMathLibrary.FindLookAtRotation` (`SceneComponent.K2_GetComponentLocation` (`self.Muzzle`)) (`SceneComponent.GetSocketLocation` (`Character.Mesh` (`GameplayStatics.GetPlayerCharacter` 0)) "spine_04")) false false))

(fn `StartAttack_RangeEnemy`
  (bind _returnvalue (`KismetMathLibrary.FindLookAtRotation` (`self.K2_GetActorLocation`) (`self.K2_GetActorLocation` (`self.PlayerRef`))))
  ; 적절한 위치를 유지하면 양옆으로 움직이며 총알 발사
  (`self.AddMovementInput` (`KismetMathLibrary.GetRightVector` _returnvalue) (`KismetMathLibrary.SelectFloat` -0.7 0.7 (`self.ChaseStrafeRight`)))
  (`self.K2_SetActorRotation` (`KismetMathLibrary.RLerp` (`self.K2_GetActorRotation`) (`KismetMathLibrary.MakeRotator` 0.0 0.0 (.yaw _returnvalue)) 0.1))
  ; 현재 공격 중이 아니면 공격
  (if (`self.bIsAttacking`)
    _
    (elif (`self.bIsReloading`)
      (bind _output_get (set `self.DeltaTimeStack` (+ (`GameplayStatics.GetWorldDeltaSeconds`) (`self.DeltaTimeStack`))))
      (if (> _output_get (`self.Enemy AttackCoolDown`))
        (set `self.bIsReloading` false)
        (set `self.DeltaTimeStack` 0.0))
      (else
        (`self.RangeEnemyOnFireEvent`)))))

(fn `UserConstructionScript`
  (`parent.UserConstructionScript`))