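; Flying ranged enemy that patrols around its spawn point and keeps attack distance from the player.
; A looping timer copies AIState to the DroneState Blackboard key, while another flips a strafe-direction flag.
; ChasePlayer advances or backs off at constant height with lerped yaw, attacking within the range band.
; FindRamdomLocation retries random points inside the patrol radius, falling back to spawn, and MoveAIToLocation steers toward a point without pathfinding.
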(event `self.ReceiveBeginPlay`
  (`parent.ReceiveBeginPlay`)
  (set `CharacterMovementComponent.MaxFlySpeed` (`self.Walk Speed`) (`self.CharacterMovement`))
  (set `self.StartLocation` (`self.K2_GetActorLocation`))
  (`KismetSystemLibrary.K2_SetTimerDelegate` (delegate `Update`) 0.2 true)
  (`self.ChaseStrafe`))

(event `Update`
  (`BlackboardComponent.SetValueAsEnum` (`self.Blackboard Component`) "DroneState" (`self.AIState`)))

(event `ChaseStrafe`
  (bind _isa (`/Engine/EditorBlueprintResources/StandardMacros.FlipFlop`)
    (:`A`
      _)
    (:`B`
      _))
  (set `self.ChaseStrafeRight` _isa)
  (`KismetSystemLibrary.K2_SetTimerDelegate` (delegate `ChaseStrafe`) 2.0))

(fn `ChasePlayer`
  (returns (Return :type Boolean))
  (bind (_returnvalue_x _returnvalue_y _returnvalue_z) (`KismetMathLibrary.BreakVector` (`self.K2_GetActorLocation`)))
  (bind (_returnvalue_x_2 _returnvalue_y_2) (`KismetMathLibrary.BreakVector` (`self.K2_GetActorLocation` (`self.PlayerRef`))))
  (bind (_returnvalue_roll _returnvalue_pitch _returnvalue_yaw) (`KismetMathLibrary.BreakRotator` (`KismetMathLibrary.FindLookAtRotation` (`self.K2_GetActorLocation`) (`KismetMathLibrary.MakeVector` _returnvalue_x_2 _returnvalue_y_2 _returnvalue_z))))
  (bind _returnvalue (`KismetMathLibrary.Conv_RotatorToVector` (`KismetMathLibrary.MakeRotator` 0.0 0.0 _returnvalue_yaw)))
  (switch `/Game/MyGame/Enemies/Enemy/Range/Ranged_Air_Enemy/E_ChaseStateEnemy` (`self.ChaseStates`)
    (:`NewEnumerator0`
      (if (> (`self.GetDistanceTo` (`GameplayStatics.GetPlayerPawn` 0)) (`self.Attack Range`))
        (`self.AddMovementInput` _returnvalue)
        (`self.K2_SetActorRotation` (`KismetMathLibrary.RLerp` (`self.K2_GetActorRotation`) (`KismetMathLibrary.MakeRotator` 0.0 0.0 _returnvalue_yaw) 0.1) :!label _label)
        (return false)
        (else
          ; 다가가면 뒤로 이동하여 사거리를 유지할려는 움직임
          (if (< (`self.GetDistanceTo` (`self.PlayerRef`)) (- (`self.Attack Range`) 100.0))
            (`self.AddMovementInput` _returnvalue -1.0)
            (goto _label)
            (else
              (`self.StartAttack_RangeEnemy`))))))))

(fn `FindRamdomLocation`
  (returns (OutLocation :type "Vector Structure"))
  (locals (TryIndex :type Integer))
  (bind (_returnvalue_x _returnvalue_y _returnvalue_z) (`KismetMathLibrary.BreakVector` (`self.K2_GetActorLocation`)))
  (bind _targetlocation (`self.TargetLocation`))
  (set `local.TryIndex` 0)
  (set `self.TargetLocation` (`KismetMathLibrary.MakeVector` (+ (`KismetMathLibrary.RandomFloatInRange` -1000.0 1000.0) _returnvalue_x) (+ (`KismetMathLibrary.RandomFloatInRange` -1000.0 1000.0) _returnvalue_y) _returnvalue_z) :!label _label)
  (if (> (`KismetMathLibrary.Abs` (`KismetMathLibrary.VSize` (- (`self.StartLocation`) (`self.TargetLocation`)))) (`self.PatrolRaius`))
    ; 실패는 10번까지
    (bind _output_get (set `local.TryIndex` (+ (`local.TryIndex`) 1)))
    (if (< _output_get 10)
      (goto _label)
      (else
        ; 최종 실패면 이동 X
        (return (`self.StartLocation`))))
    (else
      (`KismetSystemLibrary.PrintString` (`KismetStringLibrary.BuildString_Vector` "Go To" "" _targetlocation))
      ; 성공하면 그 위치로
      (return _targetlocation))))

(fn `MoveAIToLocation`
  (params (MoveToLocation :type "Vector Structure") (Threshold :type "Float (double-precision)"))
  (returns (Complete :type Boolean))
  (bind (_returnvalue_x _returnvalue_y _returnvalue_z) (`KismetMathLibrary.BreakVector` (`self.K2_GetActorLocation`)))
  (bind (_returnvalue_roll _returnvalue_pitch _returnvalue_yaw) (`KismetMathLibrary.BreakRotator` (`KismetMathLibrary.FindLookAtRotation` (`self.K2_GetActorLocation`) (`KismetMathLibrary.MakeVector` (.x MoveToLocation) (.y MoveToLocation) _returnvalue_z))))
  ; 그 위치로 가는 벡터 찾아 이동
  (if (> (`KismetMathLibrary.VSize` (- (`self.K2_GetActorLocation`) MoveToLocation)) Threshold)
    (`self.AddMovementInput` (`KismetMathLibrary.Conv_RotatorToVector` (`KismetMathLibrary.MakeRotator` 0.0 0.0 _returnvalue_yaw)) 1.0 true)
    ; 실제 액터 회전
    (`self.K2_SetActorRotation` (`KismetMathLibrary.RLerp` (`self.K2_GetActorRotation`) (`KismetMathLibrary.MakeRotator` 0.0 0.0 _returnvalue_yaw) 0.1))
    (return false)
    (else
      (return true))))

(fn `UserConstructionScript`
  (`parent.UserConstructionScript`))