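; Base enemy character that configures its movement, combat and perception stats from a data table when play begins.
; It looks up the DT_EnemyDataTable row named after its EnemyTypeTag and copies speeds, damage, attack timing and ranges into its variables.
; It then applies the walk speed to CharacterMovement and sends the type tag to its AI controller through GetEnemyTagMessage.
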(event `self.ReceiveBeginPlay`
  (`self.SetInitEnemyStats`)
  (set `CharacterMovementComponent.MaxWalkSpeed` (`self.Walk Speed`) (`self.CharacterMovement`))
  (message `/Game/Interfaces/BPI_GetEnemyStats.GetEnemyTag` (`AIBlueprintHelperLibrary.GetAIController` self) (`self.EnemyTypeTag`)))

(fn `UserConstructionScript`)