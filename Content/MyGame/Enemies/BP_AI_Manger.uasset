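; AI manager actor that spawns the level's enemies on BeginPlay.
; For each gameplay tag in EnemyTagContainer, it looks up the enemy class in DT_EnemyDataTable, using the tag name as the row name.
; It spawns that class at every TargetPoint tagged EnemySpawn, adjusting for or skipping on collision, then calls OnSpawnMessage on the enemy's AI controller.
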(event `self.ReceiveBeginPlay`
  (for _array_element (`BlueprintGameplayTagLibrary.BreakGameplayTagContainer` (`self.EnemyTagContainer`))
    (bind _returnvalue (`|GetDataTableRow` "/Game/MyGame/Enemies/Data/DT_EnemyDataTable.DT_EnemyDataTable" (`BlueprintGameplayTagLibrary.GetTagName` _array_element))
      (:`then`
        (bind _outactors (`GameplayStatics.GetAllActorsOfClassWithTag` "/Script/Engine.TargetPoint" "EnemySpawn"))
        (for _array_element_2 _outactors
          (bind _returnvalue_2 (`|SpawnActorFromClass` (`.EnemyActorClass_8_9C3D3D2F4BFBDC8C8001E7B9B0E9559B` (break `/Game/MyGame/Enemies/Data/S_EnemyData` _returnvalue)) (`self.GetTransform` _array_element_2) "AdjustIfPossibleButDontSpawnIfColliding" "MultiplyWithRoot" null null))
          (message `/Game/MyGame/Interfaces/BPI_SpawnableEnemy.OnSpawn` (`AIBlueprintHelperLibrary.GetAIController` _returnvalue_2)))))))

(fn `UserConstructionScript`)