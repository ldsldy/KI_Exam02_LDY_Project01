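; Player character Blueprint that handles Enhanced Input for moving, looking, sprinting, crouching, jumping and toggling a rifle.
; Movement follows control yaw, while sprint swaps max walk speed between two variables.
; Holding aim turns on orient-to-movement and disables turn-in-place; release restores controller-driven rotation.
; Interact sets or clears the weapon mesh and notifies the animation Blueprint, cached on BeginPlay, of equip changes.
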(event `self.ReceiveBeginPlay`
  (`self.SetAnimationBluePrintObject`))

(event `EnhancedInput|/Game/Input/IA_Aim`
  (params (ActionValue :type Boolean) (ElapsedSeconds :type "Float (double-precision)") (TriggeredSeconds :type "Float (double-precision)") (InputAction :type "InputAction Object Reference" :default "/Game/Input/IA_Aim.IA_Aim"))
  (bind _charactermovement (`self.CharacterMovement`))
  ; 견착 모드
  (:`Ongoing`
    (set `CharacterMovementComponent.bOrientRotationToMovement` true _charactermovement)
    (set `CharacterMovementComponent.bUseControllerDesiredRotation` false _charactermovement)
    (set `self.ShouldTurnInPlace` false))
  (:`Canceled`
    (set `CharacterMovementComponent.bOrientRotationToMovement` false _charactermovement :!label _label)
    (set `CharacterMovementComponent.bUseControllerDesiredRotation` true _charactermovement)
    (set `self.ShouldTurnInPlace` true))
  (:`Completed`
    (goto _label)))

(event `EnhancedInput|/Game/Input/IA_Move`
  (params (ActionValue :type "Vector2D Structure") (ElapsedSeconds :type "Float (double-precision)") (TriggeredSeconds :type "Float (double-precision)") (InputAction :type "InputAction Object Reference" :default "/Game/Input/IA_Move.IA_Move"))
  (bind (_returnvalue_roll _returnvalue_pitch _returnvalue_yaw) (`KismetMathLibrary.BreakRotator` (`self.GetControlRotation`)))
  (bind (_direction_x _direction_y) (`KismetMathLibrary.BreakVector2D` (`self.Direction`)))
  ; 걷기
  (:`Triggered`
    (set `self.Direction` (`KismetMathLibrary.MakeVector2D` ActionValue_Y ActionValue_X))
    (`self.AddMovementInput` (`KismetMathLibrary.GetForwardVector` (`KismetMathLibrary.MakeRotator` 0.0 0.0 _returnvalue_yaw)) _direction_x)
    (`self.AddMovementInput` (`KismetMathLibrary.GetRightVector` (`KismetMathLibrary.MakeRotator` 0.0 0.0 _returnvalue_yaw)) _direction_y)))

(event `EnhancedInput|/Game/Input/IA_Look`
  (params (ActionValue :type "Vector2D Structure") (ElapsedSeconds :type "Float (double-precision)") (TriggeredSeconds :type "Float (double-precision)") (InputAction :type "InputAction Object Reference" :default "/Game/Input/IA_Look.IA_Look"))
  ; 회전
  (:`Triggered`
    (`self.AddControllerYawInput` ActionValue_X)
    (`self.AddControllerPitchInput` ActionValue_Y)))

(event `EnhancedInput|/Game/Input/IA_Sprint`
  (params (ActionValue :type Boolean) (ElapsedSeconds :type "Float (double-precision)") (TriggeredSeconds :type "Float (double-precision)") (InputAction :type "InputAction Object Reference" :default "/Game/Input/IA_Sprint.IA_Sprint"))
  ; 달리기
  (:`Started`
    (`self.SetWalkSpeed` (`self.SprintSpeed`)))
  (:`Completed`
    (`self.SetWalkSpeed` (`self.MoveSpeed`))))

(event `EnhancedInput|/Game/Input/IA_Interact`
  (params (ActionValue :type Boolean) (ElapsedSeconds :type "Float (double-precision)") (TriggeredSeconds :type "Float (double-precision)") (InputAction :type "InputAction Object Reference" :default "/Game/Input/IA_Interact.IA_Interact"))
  (bind _as_abp_player_character (`self.As ABP Player Character`))
  (bind _weapon (`self.Weapon`))
  ; 무기 해제/장착
  (:`Triggered`
    (if (`self.bHasWeapon`)
      (set `self.bHasWeapon` false)
      (`/Engine/EditorBlueprintResources/StandardMacros.IsValid` (`ActorComponent.GetOwner` _weapon)
        (:`Is Valid`
          (`SkeletalMeshComponent.SetSkeletalMeshAsset` _weapon null)
          (message `/Game/Characters/BPI_WeaponSystem.OnWeaponUnequiped` _as_abp_player_character "NewEnumerator2")))
      (else
        (set `self.bHasWeapon` true)
        (`SkeletalMeshComponent.SetSkeletalMeshAsset` _weapon "/Game/Weapons/Rifle/Mesh/SK_Rifle.SK_Rifle")
        (message `/Game/Characters/BPI_WeaponSystem.OnWeaponEquiped` _as_abp_player_character "NewEnumerator0")))))

(event `EnhancedInput|/Game/Input/IA_Crouch`
  (params (ActionValue :type Boolean) (ElapsedSeconds :type "Float (double-precision)") (TriggeredSeconds :type "Float (double-precision)") (InputAction :type "InputAction Object Reference" :default "/Game/Input/IA_Crouch.IA_Crouch"))
  ; 앉기
  (:`Triggered`
    (if (not (`NavMovementInterface.IsFalling` (`self.CharacterMovement`)))
      (if (`self.bIsCrouching`)
        (`self.UnCrouch`)
        (set `self.bIsCrouching` false)
        (else
          (`self.Crouch`)
          (set `self.bIsCrouching` true))))))

(event `EnhancedInput|/Game/Input/IA_Jump`
  (params (ActionValue :type Boolean) (ElapsedSeconds :type "Float (double-precision)") (TriggeredSeconds :type "Float (double-precision)") (InputAction :type "InputAction Object Reference" :default "/Game/Input/IA_Jump.IA_Jump"))
  ; 점프
  (:`Started`
    (if (not (`NavMovementInterface.IsFalling` (`self.CharacterMovement`)))
      (`self.Jump`)
      (`KismetSystemLibrary.PrintString` "Jump"))))

(fn `SetWalkSpeed`
  (params (InSpeed :type "Float (double-precision)"))
  (set `CharacterMovementComponent.MaxWalkSpeed` InSpeed (`self.CharacterMovement`)))

(fn `UserConstructionScript`)