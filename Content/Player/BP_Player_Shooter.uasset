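; BP_Player_Shooter is a player shooter Blueprint with a prototype hitscan attack on the left mouse input action.
; When the action starts, and while it is ongoing, it line-traces on Visibility forward from the ShootingStartPoint component, leaving persistent debug lines.
; A hit on an actor tagged "Wall" only prints a message; no damage or effects are applied.
; BeginPlay, overlap and Tick hold no active logic.
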(event `EnhancedInput|/Game/Player/Input/IA_MouseLeftAttack`
  (params (ActionValue :type Boolean) (ElapsedSeconds :type "Float (double-precision)") (TriggeredSeconds :type "Float (double-precision)") (InputAction :type "InputAction Object Reference" :default "/Game/Player/Input/IA_MouseLeftAttack.IA_MouseLeftAttack"))
  (bind _returnvalue (`SceneComponent.K2_GetComponentLocation` (`self.ShootingStartPoint`)))
  (:`Started`
    (bind (_outhit _returnvalue_2) (`KismetSystemLibrary.LineTraceSingle` :`Start` _returnvalue :`End` (+ _returnvalue (* (`SceneComponent.GetForwardVector` (`self.ShootingStartPoint`)) 20000.0)) :`TraceChannel` "TraceTypeQuery1" :`DrawDebugType` "Persistent" :!label _label))
    (if _returnvalue_2
      (if (`self.ActorHasTag` (`.HitActor` (`GameplayStatics.BreakHitResult` _outhit)) "Wall")
        (`KismetSystemLibrary.PrintString` "Hit Wall"))))
  (:`Ongoing`
    (goto _label)))

(fn `UserConstructionScript`
  (`parent.UserConstructionScript`))