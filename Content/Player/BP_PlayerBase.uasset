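; Base player character Blueprint handling movement, look, sprint, crouch, jump, an aim toggle and weapon switching.
; Aim flip-flops IsHipFire and blends the view between two child-actor cameras.
; Weapon inputs equip or unequip slot classes through one ChildActor component, cycling with wraparound and caching the weapon's gameplay tag.
; It notifies ABP_PlayerCharacter of weapon changes and provides the weapon's left-hand socket in hand_r bone space.
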(event `self.ReceiveBeginPlay`
  (set `self.PlayerController` (`GameplayStatics.GetPlayerController` 0))
  (`self.SetAnimationBluePrintObject`)
  (`PlayerController.SetViewTargetWithBlend` (`self.PlayerController`) (`ChildActorComponent.ChildActor` (`self.CommonCamera`)) 0.0 "VTBlend_Linear" 0.0 false))

(event `EnhancedInput|/Game/Player/Input/IA_Aim`
  (params (ActionValue :type Boolean) (ElapsedSeconds :type "Float (double-precision)") (TriggeredSeconds :type "Float (double-precision)") (InputAction :type "InputAction Object Reference" :default "/Game/Player/Input/IA_Aim.IA_Aim"))
  ; 견착 모드
  (:`Triggered`
    (`/Engine/EditorBlueprintResources/StandardMacros.FlipFlop`
      (:`A`
        (set `self.bIsHipFire` true)
        (`PlayerController.SetViewTargetWithBlend` (`self.PlayerController`) (`ChildActorComponent.ChildActor` (`self.HipFireCamera`)) (`self.CameraBlendTime`) "VTBlend_Linear" 0.0 false)
        (`KismetSystemLibrary.Delay` (`self.CameraBlendTime`)))
      (:`B`
        (set `self.bIsHipFire` false)
        (`PlayerController.SetViewTargetWithBlend` (`self.PlayerController`) (`ChildActorComponent.ChildActor` (`self.CommonCamera`)) (`self.CameraBlendTime`) "VTBlend_Linear" 0.0 false)
        (`KismetSystemLibrary.Delay` (`self.CameraBlendTime`))))))

(event `EnhancedInput|/Game/Player/Input/IA_Move`
  (params (ActionValue :type "Vector2D Structure") (ElapsedSeconds :type "Float (double-precision)") (TriggeredSeconds :type "Float (double-precision)") (InputAction :type "InputAction Object Reference" :default "/Game/Player/Input/IA_Move.IA_Move"))
  (bind (_returnvalue_roll _returnvalue_pitch _returnvalue_yaw) (`KismetMathLibrary.BreakRotator` (`self.GetControlRotation`)))
  (bind (_direction_x _direction_y) (`KismetMathLibrary.BreakVector2D` (`self.Direction`)))
  ; 걷기
  (:`Triggered`
    (set `self.Direction` (`KismetMathLibrary.MakeVector2D` ActionValue_Y ActionValue_X))
    (`self.AddMovementInput` (`KismetMathLibrary.GetForwardVector` (`KismetMathLibrary.MakeRotator` 0.0 0.0 _returnvalue_yaw)) _direction_x)
    (`self.AddMovementInput` (`KismetMathLibrary.GetRightVector` (`KismetMathLibrary.MakeRotator` 0.0 0.0 _returnvalue_yaw)) _direction_y)))

(event `EnhancedInput|/Game/Player/Input/IA_Look`
  (params (ActionValue :type "Vector2D Structure") (ElapsedSeconds :type "Float (double-precision)") (TriggeredSeconds :type "Float (double-precision)") (InputAction :type "InputAction Object Reference" :default "/Game/Player/Input/IA_Look.IA_Look"))
  ; 회전
  (:`Triggered`
    (`self.AddControllerYawInput` ActionValue_X)
    (`self.AddControllerPitchInput` ActionValue_Y)))

(event `EnhancedInput|/Game/Player/Input/IA_Sprint`
  (params (ActionValue :type Boolean) (ElapsedSeconds :type "Float (double-precision)") (TriggeredSeconds :type "Float (double-precision)") (InputAction :type "InputAction Object Reference" :default "/Game/Player/Input/IA_Sprint.IA_Sprint"))
  ; 달리기
  (:`Started`
    (`self.SetWalkSpeed` (`self.SprintSpeed`)))
  (:`Completed`
    (`self.SetWalkSpeed` (`self.WalkSpeed`))))

(event `EnhancedInput|/Game/Player/Input/IA_Crouch`
  (params (ActionValue :type Boolean) (ElapsedSeconds :type "Float (double-precision)") (TriggeredSeconds :type "Float (double-precision)") (InputAction :type "InputAction Object Reference" :default "/Game/Player/Input/IA_Crouch.IA_Crouch"))
  (bind _charactermovement (`self.CharacterMovement`))
  ; 앉기
  (:`Triggered`
    (if (not (`NavMovementInterface.IsFalling` _charactermovement))
      (if (`NavMovementInterface.IsCrouching` _charactermovement)
        (`self.UnCrouch`)
        (else
          (`self.Crouch`))))))

(event `EnhancedInput|/Game/Player/Input/IA_Interact`
  (params (ActionValue :type Boolean) (ElapsedSeconds :type "Float (double-precision)") (TriggeredSeconds :type "Float (double-precision)") (InputAction :type "InputAction Object Reference" :default "/Game/Player/Input/IA_Interact.IA_Interact"))
  ; 무기 시스템
  ;; 무기 해제/장착
  (:`Triggered`
    (if (== (`self.CurrentWeaponTag`) (struct :`TagName` "Weapon.Type.None"))
      ;;; 무기 미장착 상태면 마지막으로 꺼냈던 무기 장착
      (`self.EquipWeapon` (`self.WeaponSlotIndex`))
      (else
        ;;; 무기 해제
        (`self.K2_DestroyActor` (`ChildActorComponent.ChildActor` (`self.Child_Weapon`)))
        (set `self.CurrentWeaponTag` (struct :`TagName` "Weapon.Type.None"))))
    ;; ABP에 무기 태그 전달
    (message `/Game/BPI/BPI_WeaponSystem.GetWeaponTagFromPlayer` (`self.As ABP Player Character`) :!label _label)))

(event `EnhancedInput|/Game/Player/Input/IA_Jump`
  (params (ActionValue :type Boolean) (ElapsedSeconds :type "Float (double-precision)") (TriggeredSeconds :type "Float (double-precision)") (InputAction :type "InputAction Object Reference" :default "/Game/Player/Input/IA_Jump.IA_Jump"))
  ; 점프
  (:`Started`
    (if (not (`NavMovementInterface.IsFalling` (`self.CharacterMovement`)))
      (`self.Jump`))))

(event `EnhancedInput|/Game/Player/Input/IA_WeaponSlot1`
  (params (ActionValue :type Boolean) (ElapsedSeconds :type "Float (double-precision)") (TriggeredSeconds :type "Float (double-precision)") (InputAction :type "InputAction Object Reference" :default "/Game/Player/Input/IA_WeaponSlot1.IA_WeaponSlot1"))
  ; 무기 시스템
  ;; 무기 스위치
  (:`Triggered`
    (bind _output_get (set `self.WeaponSlotIndex` 0))
    (`self.EquipWeapon` _output_get)
    (goto _label)))

(event `EnhancedInput|/Game/Player/Input/IA_WeaponSlot2`
  (params (ActionValue :type Boolean) (ElapsedSeconds :type "Float (double-precision)") (TriggeredSeconds :type "Float (double-precision)") (InputAction :type "InputAction Object Reference" :default "/Game/Player/Input/IA_WeaponSlot2.IA_WeaponSlot2"))
  ; 무기 시스템
  ;; 무기 스위치
  (:`Triggered`
    (bind _output_get (set `self.WeaponSlotIndex` 1))
    (`self.EquipWeapon` _output_get)
    (goto _label)))

(event `EnhancedInput|/Game/Player/Input/IA_WeaponNext`
  (params (ActionValue :type Boolean) (ElapsedSeconds :type "Float (double-precision)") (TriggeredSeconds :type "Float (double-precision)") (InputAction :type "InputAction Object Reference" :default "/Game/Player/Input/IA_WeaponNext.IA_WeaponNext"))
  ; 무기 시스템
  ;; 무기 스위치
  (:`Started`
    (bind _returnvalue (`self.SetWeaponSlotIndex` 1))
    (`self.EquipWeapon` _returnvalue)
    (goto _label)))

(event `EnhancedInput|/Game/Player/Input/IA_WeaponPrevious`
  (params (ActionValue :type Boolean) (ElapsedSeconds :type "Float (double-precision)") (TriggeredSeconds :type "Float (double-precision)") (InputAction :type "InputAction Object Reference" :default "/Game/Player/Input/IA_WeaponPrevious.IA_WeaponPrevious"))
  ; 무기 시스템
  ;; 무기 스위치
  (:`Started`
    (bind _returnvalue (`self.SetWeaponSlotIndex` -1))
    (`self.EquipWeapon` _returnvalue)
    (goto _label)))

(fn `EquipWeapon`
  (params (InIndex :type Integer))
  (bind _output (`|GetArrayItem` (`self.WeaponSlot`) InIndex))
  (`/Engine/EditorBlueprintResources/StandardMacros.IsValid` (`ChildActorComponent.ChildActor` (`self.Child_Weapon`))
    (:`Is Valid`
      (`self.K2_DestroyActor` (`ChildActorComponent.ChildActor` (`self.Child_Weapon`))))
    (:`Is Not Valid`
      _))
  ; 인벤토리에 무기가 있으면 스폰
  (if (`KismetSystemLibrary.IsValidClass` _output)
    (`ChildActorComponent.SetChildActorClass` (`self.Child_Weapon`) _output)
    ; 스폰된 무기로부터 Tag받아오기
    (bind _weapontag (message `/Game/BPI/BPI_WeaponSystem.GetWeaponTag` (`ChildActorComponent.ChildActor` (`self.Child_Weapon`))))
    (set `self.CurrentWeaponTag` _weapontag)))

(fn `GetLeftHandSocketTransform`
  (returns (LeftHandWeaponSocketTransform :type "Transform Structure"))
  (bind _childactor (`ChildActorComponent.ChildActor` (`self.Child_Weapon`)))
  (`/Engine/EditorBlueprintResources/StandardMacros.IsValid` _childactor
    (:`Is Valid`
      (bind _sockettransform (message `/Game/BPI/BPI_GetWeaponInform.GetWeaponSkeletonSocket` _childactor))
      (bind (_outposition _outrotation) (`SkinnedMeshComponent.TransformToBoneSpace` (`self.Mesh`) "hand_r" (.location _sockettransform) (.rotation _sockettransform)))
      (return (`KismetMathLibrary.MakeTransform` _outposition _outrotation)))))

(fn `SetWalkSpeed`
  (params (InSpeed :type "Float (double-precision)"))
  (set `CharacterMovementComponent.MaxWalkSpeed` InSpeed (`self.CharacterMovement`)))

(fn `SetWeaponSlotIndex`
  (params (InAddIndex :type Integer))
  (returns (ReturnValue :type Integer))
  (bind _returnvalue (`KismetArrayLibrary.Array_Length` (`self.WeaponSlot`)))
  (bind _output_get (set `self.WeaponSlotIndex` (mod (+ (+ (`self.WeaponSlotIndex`) InAddIndex) _returnvalue) _returnvalue)))
  (return _output_get))

(fn `UserConstructionScript`)